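; BP_Terminal is an in-world terminal actor that shows the text of its Terminal object on a TextRender.
; The Tab key toggles the terminal between activated and deactivated, tracking the state in an Active flag.
; The Terminal's TextUpdated event pushes each new string to the TextRender, so the Blueprint only relays input state and display output.
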(event `self.Terminal.TextUpdated`
  (params (Text :type String))
  (`TextRenderComponent.K2_SetText` (`self.TextRender`) (`KismetTextLibrary.Conv_StringToText` Text)))

(event `Key|Tab`
  (params (Key :type "Key Structure"))
  (:`Pressed`
    (if (`self.Active`)
      (`Terminal.DeactivateTerminal` (`self.Terminal`))
      (set `self.Active` false)
      (else
        (`Terminal.ActivateTerminal` (`self.Terminal`))
        (set `self.Active` true)))))

(fn `UserConstructionScript`)